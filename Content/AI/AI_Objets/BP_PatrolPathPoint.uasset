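; A patrol path point actor that turns a visiting patroller to face the direction of its Arrow component.
; OnPatrollerEntered stores the character and opens a Gate, letting Tick smoothly interpolate its rotation toward the arrow's world rotation.
; OnPatrollerExit closes the Gate when an overlap ends with the BP_AI_Enemie returned by GetActorOfClass, so only that single instance triggers it through overlap.
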(event Custom|OnPatrollerEntered
  (params (Character :type Character%20Object%20Reference))
  (Variables|Default|SetCharacter Character)
  (Utilities|FlowControl|Gate true) ; enters at Open
)

(event Custom|OnPatrollerExit
  (Utilities|FlowControl|Gate true) ; enters at Close
)

(event Collision|EventActorEndOverlap
  (params (OtherActor :type Actor%20Object%20Reference))
  (bind _returnvalue (Actor|GetActorOfClass "/Game/AI/BP_AI_Enemie.BP_AI_Enemie_C"))
  (if (== _returnvalue OtherActor)
    (CallFunction|OnPatrollerExit)))

(event EventTick
  (params (DeltaSeconds :type Float%20%28single-precision%29))
  (Utilities|FlowControl|Gate true
    (:Exit
      (Transformation|SetActorRotation (Variables|Default|GetCharacter) (Math|Interpolation|RInterpTo (Transformation|GetActorRotation (Variables|Default|GetCharacter)) (Transformation|GetWorldRotation (Variables|Default|GetArrow)) DeltaSeconds 5.0)))))

(fn ConstructionScript)