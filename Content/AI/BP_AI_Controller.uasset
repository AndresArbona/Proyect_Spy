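; AI controller that runs the BT_AI behavior tree and routes perception updates for sight, hearing and prediction into blackboard keys.
; Sight sets TargetActor to the player while seen and clears it when lost, then requests a one-second prediction of the player's position.
; The prediction stimulus writes LastKnownLocation, while heard noises from any source write TargetLocation.
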(event OnTargetPerceptionUpdated(AIPerception)
  (params (Actor :type Actor%20Object%20Reference) (Stimulus :type AI%20Stimulus%20Structure))
  (CallFunction|HandleSightSense Actor Stimulus)
  (CallFunction|HandleHearSense Stimulus)
  (CallFunction|HandlePrediction Stimulus))

(event EventBeginPlay
  (AI|RunBehaviorTree "/Game/AI/BT_AI.BT_AI"))

(fn ConstructionScript)

(fn HandleSightSense
  (params (Actor :type Actor%20Object%20Reference) (Stimulus :type AI%20Stimulus%20Structure))
  (bind _returnvalue (Class|AIPerceptionSystem|GetSenseClassforStimulus Stimulus))
  (if (== _returnvalue "/Script/AIModule.AISense_Sight")
    (if (== Actor (Game|GetPlayerCharacter 0))
      (AI|Components|Blackboard|SetValueasObject (Variables|Default|GetBlackboard) (Utilities|Name|MakeLiteralName "TargetActor") (Utilities|SelectObject (Game|GetPlayerCharacter 0) 0 (.bsuccessfullysensed Stimulus)))
      (if (not (.bsuccessfullysensed Stimulus))
        (Class|AISensePrediction|RequestPawnPredictionEvent (Pawn|GetControlledPawn) (Game|GetPlayerCharacter 0) 1.0))
      (else
        (return)))
    (else
      (return))))

(fn HandleHearSense
  (params (Stimulus :type AI%20Stimulus%20Structure))
  (bind _returnvalue (Class|AIPerceptionSystem|GetSenseClassforStimulus Stimulus))
  (if (== _returnvalue "/Script/AIModule.AISense_Hearing")
    (AI|Components|Blackboard|SetValueasVector (Variables|Default|GetBlackboard) (Utilities|Name|MakeLiteralName "TargetLocation") (.stimuluslocation Stimulus))
    (else
      (return))))

(fn HandlePrediction
  (params (Stimulus :type AI%20Stimulus%20Structure))
  (bind _returnvalue (Class|AIPerceptionSystem|GetSenseClassforStimulus Stimulus))
  (if (== _returnvalue "/Script/AIModule.AISense_Prediction")
    (AI|Components|Blackboard|SetValueasVector (Variables|Default|GetBlackboard) (Utilities|Name|MakeLiteralName "LastKnownLocation") (.stimuluslocation Stimulus))
    (else
      (return))))