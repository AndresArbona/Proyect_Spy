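; BP_NoiseTrap is a trap actor that emits an AI-detectable noise at its own location when activated.
; Tick polls IsActive and calls ActiveTrap, where a DoOnce with no reset limits it to a single firing.
; After a debug print and a short delay, it reports the noise event with itself as instigator, then clears IsActive.
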(event Custom|ActiveTrap
  (Utilities|FlowControl|DoOnce false
    (:Completed
      (Development|PrintString "Trampa Activada")
      (Utilities|FlowControl|Delay 2.0)
      (Class|AISenseHearing|ReportNoiseEvent (Transformation|GetActorLocation) 1.0 self 0.0 "None")
      (Variables|Default|SetIsActive false))))

(event EventBeginPlay)

(event Collision|EventActorBeginOverlap
  (params (OtherActor :type Actor%20Object%20Reference)))

(event EventTick
  (params (DeltaSeconds :type Float%20%28single-precision%29))
  (if (Variables|Default|GetIsActive)
    (CallFunction|ActiveTrap)))

(fn ConstructionScript)