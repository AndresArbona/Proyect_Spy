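; Player grapple component that finds a BP_GrappleTarget and pulls the character to it through a tick-driven state machine.
; While retracted, a sphere overlap plus visibility traces selects the target closest in angle to the camera's forward vector.
; AttemptGrapple spawns a hook and a hand-attached cable, turning the character toward the target.
; An upward launch follows as the hook nears, then velocity-driven pull and an exit launch before cleanup.
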(event EventBeginPlay
  ;[1 1 1] Tomamos referencia del player para usarlo en los estados
  (bind _asbp_player (Utilities|Casting|CastToBP_Player (Components|GetOwner)))
  (Variables|Private|SetOwningCharacter _asbp_player))

(event EventTick
  (params (DeltaSeconds :type Float%20%28single-precision%29))
  ;[1 1 1] Revisa en que estado esta
  (switch Utilities|FlowControl|Switch|SwitchonE_GrappleState (Variables|Private|GetGrappleState)
    (:NewEnumerator0
      (Private|TickRetracted))
    (:NewEnumerator1
      (Private|TickFiring))
    (:NewEnumerator2
      (Private|TickNearingTarget))
    (:NewEnumerator3
      (Private|TickonTarget))))

(fn TickRetracted
  (bind _outactors (Collision|SphereOverlapActors (Transformation|GetActorLocation (Variables|Private|GetOwningCharacter)) (Variables|Private|Constants|GetMaxGrappleDistance) (Utilities|Array|MakeArray "ObjectTypeQuery1") "/Game/Grapping/BP_GrappleTarget.BP_GrappleTarget_C"))
  (bind _target (Private|FindBestTarget _outactors))
  (Private|SetCurrentTarget (.AsBP%20Grapple%20Target (Utilities|Casting|CastToBP_GrappleTarget _target))))

(fn TickFiring
  (if (< (Default|DistancetoTarget (Variables|Private|GetGrappleHook)) (Variables|Private|Constants|GetStartJumpDistance))
    (Character|LaunchCharacter (Variables|Private|GetOwningCharacter) "0.000000,0.000000,500.000000" true true)
    (Variables|Private|SetGrappleState "NewEnumerator2")))

(fn TickNearingTarget
  (if (<= (.z (Transformation|GetVelocity (Variables|Private|GetOwningCharacter))) 0.0)
    (Variables|Default|SetInitialDirection (Utilities|OwnertoTarget))
    (Variables|Private|SetGrappleState "NewEnumerator3")))

(fn TickonTarget
  (bind _initialdirection (Variables|Default|GetInitialDirection))
  (bind _returnvalue (* _initialdirection 1e+02))
  (if (< (Transformation|GetDistanceTo (Variables|Private|GetOwningCharacter) (Variables|Private|GetCurrentTarget)) (Variables|Private|Constants|GetEndJumpDistance))
    (Character|LaunchCharacter (Variables|Private|GetOwningCharacter) (Math|Vector|MakeVector (.x _returnvalue) (.y _returnvalue) (Math|Float|Max(Float) (.z _returnvalue) 5e+02)) true true)
    (Private|SetCurrentTarget)
    (Actor|DestroyActor (Variables|Private|GetGrappleLine))
    (Variables|Private|SetGrappleLine 0)
    (Actor|DestroyActor (Variables|Private|GetGrappleHook))
    (Variables|Private|SetGrappleHook 0)
    (Variables|Private|SetGrappleState "NewEnumerator0")
    (else
      (Variables|/Script/Engine.MovementComponent|SetVelocity (Pawn|GetMovementComponent (Variables|Private|GetOwningCharacter)) (* (Utilities|OwnertoTarget) (Variables|Private|Constants|GetCharacterGrappleSpeed))))))

(fn FindBestTarget
  (params (Targets :type Array%20of%20Actor%20Object%20References))
  (bind _owningcharacter (Variables|Private|GetOwningCharacter))
  (bind _owningcharacter_2 (Variables|Private|GetOwningCharacter))
  ;[1 1 1] Busca entre todos los Targets disponibles y elige el mas cercano a la camara
  (for _array_element Targets
    (LocalVariables|SetCurrentTarget%28Local%29 _array_element)
    (bind (_outhit _returnvalue) (Collision|LineTraceByChannel (Transformation|GetActorLocation _owningcharacter_2) (Transformation|GetActorLocation (LocalVariables|GetCurrentTarget%28Local%29)) "TraceTypeQuery1" false (Utilities|Array|MakeArray _owningcharacter_2) "None" true "(R=1.000000,G=0.000000,B=0.000000,A=1.000000)" "(R=0.000000,G=1.000000,B=0.000000,A=1.000000)" 0.5))
    (if _returnvalue
      (if (== (.HitActor (Collision|BreakHitResult _outhit)) (LocalVariables|GetCurrentTarget%28Local%29))
        (Utilities|FlowControl|Sequence
          (:then_0
            ;[1 1 1] Paso1) Calcular el angulo hasta el objetivo
            (LocalVariables|SetCurrentAngle%28Local%29 (Class|KismetMathLibrary|DegAcos (Math|Vector|DotProduct (Math|Vector|Normalize (- (Transformation|GetActorLocation (LocalVariables|GetCurrentTarget%28Local%29)) (Transformation|GetActorLocation _owningcharacter))) (Math|Vector|GetForwardVector (Variables|/Script/Proyect_Test.CharacterClass|GetCameraComp _owningcharacter))))))
          (:then_1
            ;[1 1 1] Paso2) Si el angulo es menor que nuestro angulo actual, hacer este el nuevo angulo
            (if (or (< (LocalVariables|GetCurrentAngle%28Local%29) (LocalVariables|GetBestAngle%28Local%29)) (not (Utilities|IsValid (LocalVariables|GetBestTarget%28Local%29))))
              (LocalVariables|SetBestTarget%28Local%29 (LocalVariables|GetCurrentTarget%28Local%29))
              (LocalVariables|SetBestAngle%28Local%29 (LocalVariables|GetCurrentAngle%28Local%29))))))))
  (return (LocalVariables|GetBestTarget%28Local%29)))

(fn SetCurrentTarget
  (params (New%20Target :type BP%20Grapple%20Target%20Object%20Reference))
  (if (!= (Variables|Private|GetCurrentTarget) New%20Target)
    (Utilities|FlowControl|Sequence
      (:then_0
        (bind _currenttarget (Variables|Private|GetCurrentTarget)
          (:then
            (Default|SetActive _currenttarget false))
          (:else)))
      (:then_1
        (Variables|Private|SetCurrentTarget New%20Target))
      (:then_2
        (bind _output_get (Variables|Private|SetCurrentTarget New%20Target))
        (Default|SetActive _output_get true)))))

(fn NewFunction
  (Utilities|Casting|CastToBP_GrappleTarget (Variables|Private|GetCurrentTarget)))

(fn AttemptGrapple
  (switch Utilities|FlowControl|Switch|SwitchonE_GrappleState (Variables|Private|GetGrappleState)
    (:NewEnumerator0
      (bind _currenttarget (Variables|Private|GetCurrentTarget)
        (:then
          (bind _returnvalue (Game|SpawnActorfromClass "/Game/Grapping/BP_GrappleHook.BP_GrappleHook_C" (Math|Transform|MakeTransform (Utilities|OwnweLocation) "0, 0, 0" "1.000000,1.000000,1.000000") "AlwaysSpawn" 0 _currenttarget 5e+03 0))
          (Variables|Private|SetGrappleHook _returnvalue)
          (bind _returnvalue_2 (Game|SpawnActorfromClass "/Game/Grapping/BP_GrappleLine.BP_GrappleLine_C" (Math|Transform|MakeTransform (Utilities|OwnweLocation) "0, 0, 0" "1.000000,1.000000,1.000000") "AlwaysSpawn" 0 0))
          (bind _output_get (Variables|Private|SetGrappleLine _returnvalue_2))
          (Transformation|AttachComponentToComponent _output_get (Variables|/Script/Engine.Character|GetMesh (Variables|Private|GetOwningCharacter)) "hand_r" "SnapToTarget" "SnapToTarget" "SnapToTarget" true)
          (Class|CableComponent|SetAttachEndto (Variables|/Script/CableComponent.CableActor|GetCableComponent (Variables|Private|GetGrappleLine)) (Variables|Private|GetGrappleHook) "DefaultSceneRoot" "None")
          (Transformation|SetActorRotation (Variables|Private|GetOwningCharacter) (Math|Rotator|MakeRotfromZX (Math|Vector|MakeVector 0.0 0.0 1.0) (Utilities|OwnertoTarget)))
          (Variables|Private|SetGrappleState "NewEnumerator1"))
        (:else)))))