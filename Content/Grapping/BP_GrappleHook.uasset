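; BP_GrappleHook is a grapple hook projectile that flies from its spawn point to a Target and stops there.
; On BeginPlay it caches start and end locations and launches its ProjectileMovement along that direction.
; Tick compares squared distances from the start to detect reaching or passing the Target, then snaps to the cached endpoint and zeroes velocity.
; DistanceToTarget reports the remaining distance to that endpoint.
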(event EventBeginPlay
  (Variables|Private|SetStartingLocation (Transformation|GetActorLocation))
  (Variables|Private|SetEndingLocation (Transformation|GetActorLocation (Variables|Private|GetTarget)))
  (Variables|Default|SetDirection (Math|Vector|Normalize (- (Variables|Private|GetEndingLocation) (Variables|Private|GetStartingLocation))))
  (Variables|/Script/Engine.MovementComponent|SetVelocity (Variables|Default|GetProjectileMovement) (* (Variables|Default|GetDirection) (Variables|Default|GetVelocity))))

(event EventTick
  (params (DeltaSeconds :type Float%20%28single-precision%29))
  (if (>= (Class|KismetMathLibrary|VectorDistanceSquared (Transformation|GetActorLocation) (Variables|Private|GetStartingLocation)) (Class|KismetMathLibrary|VectorDistanceSquared (Transformation|GetActorLocation (Variables|Private|GetTarget)) (Variables|Private|GetStartingLocation)))
    (Transformation|SetActorLocation (+ (Variables|Private|GetStartingLocation) (* (Variables|Default|GetDirection) (Math|Vector|Distance(Vector) (Variables|Private|GetStartingLocation) (Variables|Private|GetEndingLocation)))) false false)
    (Variables|/Script/Engine.MovementComponent|SetVelocity (Variables|Default|GetProjectileMovement) "0, 0, 0")))

(fn ConstructionScript)

(fn DistancetoTarget
  (return (Math|Vector|Distance(Vector) (Variables|Private|GetEndingLocation) (Transformation|GetActorLocation))))